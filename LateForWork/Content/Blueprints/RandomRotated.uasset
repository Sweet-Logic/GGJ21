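; RandomRotated is a placeable static mesh actor that gives itself a random orientation for varied prop placement.
; The construction script applies the StaticMesh variable to the Mesh component.
; When Rotate is true, it adds a random full-circle offset to roll, pitch and yaw, then clears the flag so it works as a one-shot toggle.
; The event graph has no active logic.
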(fn `UserConstructionScript`
  (bind (_returnvalue_roll _returnvalue_pitch _returnvalue_yaw) (`KismetMathLibrary.BreakRotator` (`self.K2_GetActorRotation`)))
  (bind _returnvalue (`KismetMathLibrary.RandomFloatInRange` 0.0 360.0))
  (`StaticMeshComponent.SetStaticMesh` (`self.mesh`) (`self.Static Mesh`))
  (if (`self.rotate`)
    (`self.K2_SetActorRotation` (`KismetMathLibrary.MakeRotator` (+ _returnvalue_roll _returnvalue) (+ _returnvalue_pitch _returnvalue) (+ _returnvalue_yaw _returnvalue)))
    (set `self.rotate` false)))